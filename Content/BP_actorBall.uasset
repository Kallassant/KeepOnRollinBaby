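; Ball actor that moves itself along a direction vector, bouncing and losing speed on impacts.
; Tick moves the sphere with a swept world offset, and a blocking hit recomputes Direction via GetReflectionVector, with hit normal and Direction in swapped inputs.
; Both that bounce and the Hit event call the slowdown function, which multiplies speed by a slowdown factor while it is at or above the minimum.
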(event `self.ReceiveTick`
  (params (DeltaSeconds :type "Float (single-precision)"))
  (bind _sweephitresult (`SceneComponent.K2_AddWorldOffset` (`self.Sphere`) (* DeltaSeconds (* (`self.SpeedBase`) (`self.Direction`))) true false))
  (bind (_bblockinghit _binitialoverlap _time _distance _location _impactpoint _normal) (`GameplayStatics.BreakHitResult` _sweephitresult))
  (if _bblockinghit
    (set `self.Direction` (`KismetMathLibrary.GetReflectionVector` _normal (`self.Direction`)))
    (`self.Ball Slows Down (10% for each hit)` :!label _label)))

(event `self.ReceiveHit`
  (params (MyComp :type "PrimitiveComponent Object Reference") (Other :type "Actor Object Reference") (OtherComp :type "PrimitiveComponent Object Reference") (bSelfMoved :type Boolean) (HitLocation :type "Vector Structure") (HitNormal :type "Vector Structure") (NormalImpulse :type "Vector Structure") (Hit :type "HitResult Structure (by ref)"))
  (goto _label))

(fn `Ball Slows Down (10% for each hit)`
  (if (>= (`self.SpeedBase`) (`self.SpeedMinimum`))
    (set `self.SpeedBase` (* (`self.SpeedBase`) (`self.SpeedSlowdown`)))))

(fn `UserConstructionScript`)