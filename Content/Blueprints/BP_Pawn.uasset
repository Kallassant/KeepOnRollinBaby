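; BP_Pawn is a player pawn that spawns a ball and slides sideways on the Move Right and Left axis.
; On BeginPlay it spawns BP_InGameBall at its Sphere's transform, stores it as PlayingBall and binds to its OnDead.
; Input moves the actor along Y in fixed swept steps per event, unscaled by delta time.
; Tick sweeps the Cube with a zero offset and clears Direction on a blocking hit.
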(event `self.ReceiveBeginPlay`
  (`self.SpawnBall`))

(event `self.ReceiveTick`
  (params (DeltaSeconds :type "Float (single-precision)"))
  (bind _sweephitresult (`SceneComponent.K2_AddWorldOffset` (`self.Cube`) (0.0 0.0 0.0) true false))
  (if (`GameplayStatics.BreakHitResult` _sweephitresult)
    (set `self.Direction` (0.0 0.0 0.0))))

(event `InputAxis|Move Right and Left`
  (params (AxisValue :type "Float (single-precision)"))
  (if (< AxisValue 0.0)
    (`self.K2_AddActorWorldOffset` (0.0 50.0 0.0) true)))

(event `InputAxis|Move Right and Left`
  (params (AxisValue :type "Float (single-precision)"))
  (if (> AxisValue 0.0)
    (`self.K2_AddActorWorldOffset` (0.0 -50.0 0.0) true)))

(fn `SpawnBall`
  (bind _returnvalue (`|SpawnActorFromClass` "/Game/Blueprints/BP_InGameBall.BP_InGameBall_C" (`SceneComponent.K2_GetComponentToWorld` (`self.Sphere`)) "AlwaysSpawn" "MultiplyWithRoot" null null))
  (bind _output_get (set `self.PlayingBall` _returnvalue))
  (add `/Game/Blueprints/BP_actorBall.OnDead` _output_get (`|CreateDelegate` :!event `SpawnBall`)))

(fn `UserConstructionScript`)